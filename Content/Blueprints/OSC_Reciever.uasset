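; OSC receiver that lets two external controllers move the Player 1 and Player 2 actors.
; BeginPlay starts one OSC server per player on separate ports; each handles "/shark Move" messages.
; Two floats are remapped to -1..1, then scaled and inverted into world X/Y offsets per message.
; The intended dead zone's AND condition never passes, so it has no effect; Player 3 and 4 setup is unconnected, with empty handlers.
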(event Custom|OSCMessageP2Received
  (params (Message :type OSC%20Message%20Structure%20%28by%20ref%29) (IPAddress :type String) (Port :type Integer))
  ;[1 1 1] Control Player 2
  (bind _returnvalue (Class|OSCManager|GetOSCMessageAddress Message))
  (bind _returnvalue_2 (Class|OSCManager|GetOSCAddressFullPath _returnvalue))
  (switch string _returnvalue_2
    (:/sharkMove
      (CallFunction|P2Move))))

(event Custom|OSCMessageReceived
  (params (Message :type OSC%20Message%20Structure%20%28by%20ref%29) (IPAddress :type String) (Port :type Integer))
  ;[1 1 1] Control Player 1
  (bind _returnvalue (Class|OSCManager|GetOSCMessageAddress Message))
  (bind _returnvalue_2 (Class|OSCManager|GetOSCAddressFullPath _returnvalue))
  (switch string _returnvalue_2
    (:/sharkMove
      (CallFunction|MoveShark))))

(event Custom|moveShark
  ;[1 1 1] Control Player 1
  (bind _value (Class|OSCManager|GetFloat (stale Custom|OSCMessageReceived Message)))
  (bind _value_2 (Class|OSCManager|GetFloat (stale Custom|OSCMessageReceived Message) 1))
  (Class|Actor|AddActorWorldTransform (Variables|Default|GetP1MovableActor) (Math|Transform|MakeTransform (Math|Vector|MakeVector (* (Math|Float|SelectFloat 0.0 (Math|Float|MapRangeClamped _value_2 0.0 1.0 -1.0 1.0) (and (> (Math|Float|MapRangeClamped _value_2 0.0 1.0 -1.0 1.0) 0.1) (< (Math|Float|MapRangeClamped _value_2 0.0 1.0 -1.0 1.0) -0.1))) -2.0) (* (Math|Float|SelectFloat 0.0 (Math|Float|MapRangeClamped _value 0.0 1.0 -1.0 1.0) (and (> (Math|Float|MapRangeClamped _value 0.0 1.0 -1.0 1.0) 0.1) (< (Math|Float|MapRangeClamped _value 0.0 1.0 -1.0 1.0) -0.1))) -2.0) 0.0) "0, 0, 0" "1.000000,1.000000,1.000000") false false))

(event Custom|OSCMessageP3Received
  (params (Message :type OSC%20Message%20Structure%20%28by%20ref%29) (IPAddress :type String) (Port :type Integer)))

(event Custom|OSCMessageP4Received
  (params (Message :type OSC%20Message%20Structure%20%28by%20ref%29) (IPAddress :type String) (Port :type Integer)))

(event Custom|P2%20Move
  ;[1 1 1] Control Player 2
  (bind _value (Class|OSCManager|GetFloat (stale Custom|OSCMessageP2Received Message)))
  (bind _value_2 (Class|OSCManager|GetFloat (stale Custom|OSCMessageP2Received Message) 1))
  (Class|Actor|AddActorWorldTransform (Variables|Default|GetP2MovableActor) (Math|Transform|MakeTransform (Math|Vector|MakeVector (* (Math|Float|SelectFloat 0.0 (Math|Float|MapRangeClamped _value_2 0.0 1.0 -1.0 1.0) (and (> (Math|Float|MapRangeClamped _value_2 0.0 1.0 -1.0 1.0) 0.1) (< (Math|Float|MapRangeClamped _value_2 0.0 1.0 -1.0 1.0) -0.1))) -2.0) (* (Math|Float|SelectFloat 0.0 (Math|Float|MapRangeClamped _value 0.0 1.0 -1.0 1.0) (and (> (Math|Float|MapRangeClamped _value 0.0 1.0 -1.0 1.0) 0.1) (< (Math|Float|MapRangeClamped _value 0.0 1.0 -1.0 1.0) -0.1))) -2.0) 0.0) "0, 0, 0" "1.000000,1.000000,1.000000") false false))

(event EventBeginPlay
  ;[1 1 1] OSC Server Player 1
  (bind _returnvalue (Class|OSCManager|CreateOSCServer (Variables|Default|GetIP-Adress) 8080 false true "" 0))
  (bind _output_get (Variables|Default|SetOSCServerP1 _returnvalue))
  (EventDispatchers|UnbindallEventsfromOnOscBundleReceived _output_get)
  (EventDispatchers|BindEventtoOnOscMessageReceived _output_get (EventDispatchers|CreateEvent :!event Custom|OSCMessageReceived))
  ;[1 1 1] OSC Server Player 2
  (bind _returnvalue_2 (Class|OSCManager|CreateOSCServer (Variables|Default|GetIP-Adress) 8069 false true "" 0))
  (bind _output_get_2 (Variables|Default|SetOSCServerP2 _returnvalue_2))
  (EventDispatchers|UnbindallEventsfromOnOscBundleReceived _output_get_2)
  (EventDispatchers|BindEventtoOnOscMessageReceived _output_get_2 (EventDispatchers|CreateEvent :!event Custom|OSCMessageP2Received)))

(fn ConstructionScript)